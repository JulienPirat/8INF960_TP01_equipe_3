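; BP_Player is the player-controlled paddle for a brick-breaker game, moving only left and right.
; On BeginPlay it adds the QWERTY Enhanced Input mapping context to player controller 0.
; The IA_Move action offsets the Paddle component with a swept local offset along its right vector, scaled by the input value and Vitesse, and prints the value for debugging.
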(event Input|EnhancedActionEvents|EnhancedInputActionIA_Move
  (params (ActionValue :type Float%20%28double-precision%29) (ElapsedSeconds :type Float%20%28double-precision%29) (TriggeredSeconds :type Float%20%28double-precision%29) (InputAction :type Input%20Action%20Object%20Reference :default "/Game/CasseBrique_RPMC/Inputs/IA_Move.IA_Move"))
  (bind _paddle (Variables|Default|GetPaddle))
  ;[1 1 1] On ajoute les mouvement (Y'a que du gauche droite)
  (:Triggered
    (Development|PrintString (Utilities|String|ToString(Float) ActionValue))
    (Transformation|AddLocalOffset _paddle (* ActionValue (Math|Vector|GetRightVector _paddle) (Variables|Default|GetVitesse)) true false)))

(event EventBeginPlay
  ;[1 1 1] On ajoute les touches définis aux joueurs
  (bind _asplayer_controller (Utilities|Casting|CastToPlayerController (Game|GetPlayerController 0)))
  (Utilities|IsValid (PlayerController|LocalPlayerSubsystems|GetEnhancedInputLocalPlayerSubsystem _asplayer_controller)
    (:Is%20Valid
      (Input|AddMappingContext (PlayerController|LocalPlayerSubsystems|GetEnhancedInputLocalPlayerSubsystem _asplayer_controller) "/Game/CasseBrique_RPMC/Inputs/IMC_QWERTY.IMC_QWERTY" 0 "(bIgnoreAllPressedKeysUntilRelease=True,bForceImmediately=False)"))))

(fn ConstructionScript)